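; BP_PickupAmmoBase is the base ammo pickup that gives the FPS character ammo of a configured weapon type when walked over.
; On the parent's character overlap event, it asks the inventory whether that ammo type can be taken, then adds the configured count and destroys itself.
; If the inventory cannot take it, the pickup stays in the world.
; Its sphere rotates a fixed step every tick, independent of delta time.
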(event EventBeginPlay
  (|CallParentFunction) ; This node is disabled and will not be called.\nDrag off pins to build functionality.
)

(event EventOverlapFPSCharacter
  (params (Inventory :type Inventory%20Component%20Object%20Reference) (CharHealthComp :type Char%20Health%20Component%20Object%20Reference))
  (bind _weapontypeammo (Variables|Default|GetWeaponTypeAmmo))
  (|CallParentFunction Inventory CharHealthComp)
  (bind _returnvalue (Class|InventoryComponent|CheckCanTakeAmmo Inventory _weapontypeammo))
  (if _returnvalue
    (Class|InventoryComponent|AmmoSlotChangeValue Inventory _weapontypeammo (Variables|Default|GetCount))
    (Actor|DestroyActor)))

(event EventTick
  (params (DeltaSeconds :type Float%20%28single-precision%29))
  (Transformation|AddLocalRotation (Variables|Default|GetSphere) "0,1.000000, 0" false false))

(fn ConstructionScript
  (|CallParentFunction))