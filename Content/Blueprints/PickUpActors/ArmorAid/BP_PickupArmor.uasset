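; BP_PickupArmor is an armor pickup that restores shield to the FPS character who overlaps it.
; On overlap, it reads the character's health component and, only if shield is below a hard-coded cap, applies ShieldValue, plays a 2D sound and destroys itself.
; A full-shield character leaves the pickup in place.
; Tick spins the Sphere component by a fixed step each frame, independent of delta time.
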(event EventBeginPlay
  (|CallParentFunction) ; This node is disabled and will not be called.\nDrag off pins to build functionality.
)

(event EventTick
  (params (DeltaSeconds :type Float%20%28single-precision%29))
  (Transformation|AddRelativeRotation (Variables|Default|GetSphere) "0,1.000000, 0" false false))

(event EventOverlapFPSCharacter
  (params (Inventory :type Inventory%20Component%20Object%20Reference) (CharHealthComp :type Char%20Health%20Component%20Object%20Reference))
  (bind _returnvalue (Class|CharHealthComponent|GetCurrentShield CharHealthComp))
  (if (< _returnvalue 1e+02)
    (Class|CharHealthComponent|ChangeShieldValue CharHealthComp (Variables|Default|GetShieldValue))
    (Audio|PlaySound2D "/Game/Blueprints/PickUpActors/FirstAid/HealSound.HealSound" 1.0 1.0 0.0 0 0)
    (Actor|DestroyActor)))

(fn ConstructionScript
  (|CallParentFunction))