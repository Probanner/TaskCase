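; Base weapon pickup that spins in the world and gives a weapon or ammo to an overlapping FPS character.
; The construction script sets its slot data and skeletal mesh from configured variables.
; After a short overlap delay, it adds ammo for an already-owned weapon name, otherwise tries adding the weapon, destroying itself when taken.
; Hitting anything except another pickup stops sphere physics, hovers it above the impact and enables overlaps.
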(event OnComponentHit(Sphere)
  (params (HitComponent :type Primitive%20Component%20Object%20Reference) (OtherActor :type Actor%20Object%20Reference) (OtherComp :type Primitive%20Component%20Object%20Reference) (NormalImpulse :type Vector :default "0, 0, 0") (Hit :type Hit%20Result%20Structure%20%28by%20ref%29))
  (bind (_bblockinghit _binitialoverlap _time _distance _location _impactpoint _normal _impactnormal _physmat _hitactor) (Collision|BreakHitResult Hit))
  (bind _sphere (Variables|Default|GetSphere))
  (Utilities|Casting|CastToBP_PickupActorBase _hitactor
    (:CastFailed
      (Physics|SetSimulatePhysics _sphere false)
      (Transformation|SetWorldLocation _sphere (Math|Vector|MakeVector (.x _impactpoint) (.y _impactpoint) (+ (.z _impactpoint) 5e+01)) false false)
      (Transformation|SetRelativeRotation (Variables|Default|GetSphere) "0, 0, 0" false false)
      (Variables|/Script/Engine.PrimitiveComponent|SetbGenerateOverlapEvents _sphere true))))

(event EventBeginPlay
  (|CallParentFunction) ; This node is disabled and will not be called.\nDrag off pins to build functionality.
)

(event Collision|EventActorBeginOverlap
  (params (OtherActor :type Actor%20Object%20Reference)))

(event EventTick
  (params (DeltaSeconds :type Float%20%28single-precision%29))
  (Transformation|AddWorldRotation (Variables|Default|GetSphere) "0,-1.000000, 0" false false))

(event EventOverlapFPSCharacter
  (params (Inventory :type Inventory%20Component%20Object%20Reference) (CharHealthComp :type Char%20Health%20Component%20Object%20Reference))
  (|CallParentFunction Inventory CharHealthComp)
  (Utilities|FlowControl|Delay 0.2)
  (Variables|Default|SetbIsSame false)
  (for _array_element (Variables|/Script/TaskCase.InventoryComponent|GetWeaponSlots Inventory)
    (if (Utilities|Name|Equal(Name) (.ItemName (Utilities|Struct|BreakWeaponSlot _array_element)) (.ItemName (Utilities|Struct|BreakWeaponSlot (Variables|Default|GetWeaponSlotByDefault))))
      (Variables|Default|SetbIsSame true)
      (if (not (Variables|Default|GetbTakeAmmoSameWeapon))
        (CallFunction|TakeAmmoSameWeapon Inventory (.WeaponType (Utilities|Struct|BreakWeaponSlot _array_element))))))
  (if (not (Variables|Default|GetbIsSame))
    (bind _returnvalue (Class|InventoryComponent|TryGetWeapontoInventory Inventory (Variables|Default|GetWeaponSlotByDefault)))
    (if _returnvalue
      (Actor|DestroyActor))))

(fn ConstructionScript
  (bind _weaponslotbyconstruct (Variables|Default|GetWeaponSlotByConstruct))
  (bind (_itemname _weapontype _additionalinfo) (Utilities|Struct|BreakWeaponSlot _weaponslotbyconstruct))
  (|CallParentFunction)
  (if (Utilities|Name|Equal(Name) _itemname "None")
    (Development|PrintString "WrongName")
    (else
      (Variables|Default|SetWeaponSlotByDefault (Utilities|Struct|MakeWeaponSlot _itemname _weapontype _additionalinfo))
      (Class|SkinnedMeshComponent|SetSkeletalMesh (Variables|Default|GetSkeletalMesh) (Variables|Default|GetSkeletalByConstruct) true)
      (Development|PrintString (Utilities|String|ToString(Integer) (Utilities|Struct|BreakAdditionalWeaponInfo _additionalinfo))))))

(fn TakeAmmoSameWeapon
  (params (Inventory :type Inventory%20Component%20Object%20Reference) (WeaponType :type EWeaponType%20Enum :default "RifleType"))
  (for _array_element (Variables|/Script/TaskCase.InventoryComponent|GetAmmoSlots Inventory)
    (if (Utilities|Enum|Equal(Enum) (.WeaponType (Utilities|Struct|BreakAmmoSlot _array_element)) WeaponType)
      (if (!= (.Count (Utilities|Struct|BreakAmmoSlot _array_element)) (.MaxCount (Utilities|Struct|BreakAmmoSlot _array_element)))
        (Variables|Default|SetbTakeAmmoSameWeapon true)
        (Class|InventoryComponent|AmmoSlotChangeValue Inventory WeaponType (Variables|Default|GetAddAmmoIfSameWeapon))
        (Actor|DestroyActor))
      (else
        (bind _returnvalue (Class|InventoryComponent|CheckCanTakeAmmo Inventory WeaponType))
        (if _returnvalue
          (Class|InventoryComponent|AmmoSlotChangeValue Inventory WeaponType 10))))))