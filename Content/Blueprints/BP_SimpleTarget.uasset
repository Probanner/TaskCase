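; BP_SimpleTarget is a simple damageable target actor that is destroyed when its Health component reports death.
; AnyDamage passes damage to Health as a negative change, only while current health is above zero.
; BeginPlay binds the component's death and health-change events.
; An OnHealthChange handler prints the negated damage value, and the auto-generated function is an empty stub.
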(event Custom|OnDead
  (Actor|DestroyActor))

(event Custom|OnHealthChange
  (params (Health :type Float%20%28single-precision%29) (Damage :type Float%20%28single-precision%29))
  (Development|PrintString (Utilities|String|ToString(Float) (* -1 Damage))))

(event Game|Damage|EventAnyDamage
  (params (Damage :type Float%20%28single-precision%29) (DamageType :type Damage%20Type%20Object%20Reference) (InstigatedBy :type Controller%20Object%20Reference) (DamageCauser :type Actor%20Object%20Reference))
  (bind _returnvalue (Class|HealthComponent|GetCurrentHealth (Variables|Default|GetHealth)))
  (if (> _returnvalue 0.0)
    (Class|HealthComponent|ChangeCurrentHealth (Variables|Default|GetHealth) (* -1 Damage))))

(event EventBeginPlay
  (EventDispatchers|BindEventtoOnDead (Variables|Default|GetHealth) (delegate Custom|OnDead))
  (EventDispatchers|BindEventtoOnHeathChange (Variables|Default|GetHealth) (EventDispatchers|CreateEvent :!event Custom|OnHealthChange)))

(fn ConstructionScript)

(fn BPTargetAutoGenFunc
  (params (Health :type Float%20%28single-precision%29) (Damage :type Float%20%28single-precision%29)))